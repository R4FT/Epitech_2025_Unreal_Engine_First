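; BP_Ammo is an ammo pickup for one fixed weapon type, collected when the player touches its box.
; On overlap it confirms the actor is BP_Player, owns a weapon of that type and is not already at max ammo.
; It then passes its Ammo amount to the player's TakeAmmo, plays a 2D pickup sound and destroys itself; otherwise it stays in the world.
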(event OnComponentBeginOverlap(Box)
  (params (OverlappedComponent :type Primitive%20Component%20Object%20Reference) (OtherActor :type Actor%20Object%20Reference) (OtherComp :type Primitive%20Component%20Object%20Reference) (OtherBodyIndex :type Integer) (bFromSweep :type Boolean) (SweepResult :type Hit%20Result%20Structure%20%28by%20ref%29))
  (bind _asbp_player (Utilities|Casting|CastToBP_Player OtherActor))
  (bind _hasweaponoftype (Default|GetWeaponOfType _asbp_player "NewEnumerator2"))
  (if _hasweaponoftype
    (bind _currentweaponoftype (Default|GetWeaponOfType _asbp_player "NewEnumerator2"))
    (if (!= (Variables|/Game/Props/Weapons/BP_WeaponMaster.BP_WeaponMaster_C|GetAmmo _currentweaponoftype) (Variables|/Game/Props/Weapons/BP_WeaponMaster.BP_WeaponMaster_C|GetMaxAmmo _currentweaponoftype))
      (Default|TakeAmmo _asbp_player (Variables|Default|GetAmmo) "NewEnumerator2")
      (Audio|PlaySound2D "/Game/Sound/Ammo_Pickup.Ammo_Pickup" 1.0 1.0 0.0 0 0)
      (Actor|DestroyActor))))

(fn ConstructionScript)