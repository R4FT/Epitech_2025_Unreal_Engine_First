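; BP_Enemy is a zombie enemy for a wave-based game that chases the player and damages them on contact.
; While it sees the player, Tick reissues an AI MoveTo toward them, pausing briefly after each capsule-overlap hit.
; Incoming damage drains Life and plays sounds.
; On death it updates the Bp_WaveZombies game mode's round count, delegates death and consumable spawning to BPDeath, and awards score.
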(event OnComponentBeginOverlap(Capsule)
  (params (OverlappedComponent :type Primitive%20Component%20Object%20Reference) (OtherActor :type Actor%20Object%20Reference) (OtherComp :type Primitive%20Component%20Object%20Reference) (OtherBodyIndex :type Integer) (bFromSweep :type Boolean) (SweepResult :type Hit%20Result%20Structure%20%28by%20ref%29))
  (bind _asbp_player (Utilities|Casting|CastToBP_Player OtherActor))
  (Default|TakeDamage _asbp_player 25)
  (Variables|Default|SetIsSeeingPlayer false)
  (Utilities|FlowControl|Delay 1.0)
  (Variables|Default|SetIsSeeingPlayer true))

(event Custom|Follow%20Player
  (AI|AIMoveTo self "0, 0, 0" (Game|GetPlayerCharacter 0) 5.0 false))

(event EventTick
  (params (DeltaSeconds :type Float%20%28single-precision%29))
  (if (Variables|Default|GetIsSeeingPlayer)
    (CallFunction|FollowPlayer)))

(event Game|Damage|EventAnyDamage
  (params (Damage :type Float%20%28single-precision%29) (DamageType :type Damage%20Type%20Object%20Reference) (InstigatedBy :type Controller%20Object%20Reference) (DamageCauser :type Actor%20Object%20Reference))
  (bind _bp_sound (Variables|Default|GetBP_Sound))
  (bind _output_get (Variables|Default|SetLife (- (Variables|Default|GetLife) Damage)))
  (if (> _output_get 0.0)
    (Default|PlaySoundDamage _bp_sound)
    (else
      (Default|PlayDeathDamage _bp_sound)
      (bind _asbp_wave_zombies (Utilities|Casting|CastToBp_WaveZombies (Game|GetGameMode)))
      (Math|Integer|DecrementInt (Variables|/Game/Player/Bp_WaveZombies.Bp_WaveZombies_C|GetZombies_Alive _asbp_wave_zombies)
        (:%20%20
          (Default|CheckRoundEnd _asbp_wave_zombies)
          (Default|DeathEnnemy (Variables|Default|GetBP_Death) (Variables|Default|GetSpawnConsumable) self)
          (bind _asbp_player (Utilities|Casting|CastToBP_Player (Game|GetPlayerCharacter 0)))
          (Default|AddScore _asbp_player 100))))))

(fn ConstructionScript)