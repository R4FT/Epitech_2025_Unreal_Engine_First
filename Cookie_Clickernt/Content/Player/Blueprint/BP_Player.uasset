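; Third-person player character with Enhanced Input movement, camera aim zoom, a grappling hook, health with respawn at the start transform, and a HUD.
; Weapons live in a map keyed by type; pickups spawn and attach them, and equip montage notifies toggle their visibility.
; Firing uses line traces from the barrel, with ten random-spread pellets for the shotgun, and montage-driven reloads refill the magazine from reserve ammo.
; The grapple pulls the player in Flying mode along a visible cable.
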(event Custom|SetInputMappingContext
  ;[0.8717 1 0.3181] Movement
  (bind _asplayer_controller (Utilities|Casting|CastToPlayerController (Pawn|GetController)))
  (Utilities|IsValid (PlayerController|LocalPlayerSubsystems|GetEnhancedInputLocalPlayerSubsystem _asplayer_controller)
    (:Is%20Valid
      (Input|AddMappingContext (PlayerController|LocalPlayerSubsystems|GetEnhancedInputLocalPlayerSubsystem _asplayer_controller) "/Game/Player/Input/InputMapping/My_Mapping.My_Mapping" 0 "(bIgnoreAllPressedKeysUntilRelease=True,bForceImmediately=False,bNotifyUserSettings=False)")
      (bind _returnvalue (Game|ConstructObjectfromClass "/Game/Player/UserInterface/WB_HUD.WB_HUD_C"))
      (UserInterface|Viewport|AddtoViewport _returnvalue 0))))

(event Custom|TakeDamage
  (params (Damage :type Integer))
  ;[1 0.009744 0] Damage
  (Variables|Default|SetLife (- (Variables|Default|GetLife) Damage))
  (if (> (Variables|Default|GetLife) 0)
    (Default|PlaySoundDamage (Variables|Default|GetBP_Sound))
    (else
      (CallFunction|Die))))

(event Custom|Equip%20weapon
  (params (New%20weapon :type Enum_WeaponType%20Enum :default "NewEnumerator0"))
  ;[1 1 1] Equip weapon from inventory
  (bind _ispresent (CallFunction|TakeWeapon New%20weapon))
  (if (== _ispresent true)
    (Animation|Montage|PlayMontage (Variables|Character|GetMesh) "/Game/Animation/AM_EquipRifle.AM_EquipRifle" 1.4
      (:then
        (bind _currentweapon (CallFunction|GetCurrentWeapon))
        (Variables|Default|SetCurrentWeaponEnum (Variables|/Game/Props/Weapons/BP_WeaponMaster.BP_WeaponMaster_C|GetWeaponName _currentweapon)))
      (:OnCompleted
        (Variables|Default|SetCanFire true))
      (:OnNotifyBegin
        (CallFunction|SetWeaponVisibility)))))

(event Custom|Die
  ;[1 0.1453 0.1751] Death
  (Default|PlayDeathDamage (Variables|Default|GetBP_Sound))
  (Utilities|FlowControl|Delay 0.2)
  (Transformation|SetActorTransform (Variables|Default|GetSpawnPosition) false true)
  (Variables|Default|SetLife (Variables|Default|GetMaxLife)))

(event Custom|setSpawnPosition
  ;[1 0.1453 0.1751] Death
  (Variables|Default|SetSpawnPosition (Transformation|GetActorTransform)))

(event Custom|Aim%20Forward
  (bind _charactermovement (Variables|Character|GetCharacterMovement))
  ;[1 1 1] Aim Logic
  (Variables|/Script/Engine.CharacterMovementComponent|SetbOrientRotationToMovement _charactermovement false)
  (Variables|/Script/Engine.CharacterMovementComponent|SetbUseControllerDesiredRotation _charactermovement true))

(event Custom|Stop%20Aim%20Forward
  (bind _charactermovement (Variables|Character|GetCharacterMovement))
  ;[1 1 1] Aim Logic
  (Variables|/Script/Engine.CharacterMovementComponent|SetbOrientRotationToMovement _charactermovement true)
  (Variables|/Script/Engine.CharacterMovementComponent|SetbUseControllerDesiredRotation _charactermovement false))

(event Custom|TakeHeal
  (params (Health :type Integer))
  ;[1 1 1] Heal
  (Variables|Default|SetLife (Math|Integer|Clamp(Integer) (+ Health (Variables|Default|GetLife)) 0 (Variables|Default|GetMaxLife)))
  (Default|PlayHealSound (Variables|Default|GetBP_Sound)))

(event Custom|SpawnWeapon
  (params (WeaponToSpawn :type BP%20Weapon%20Master%20Class%20Reference) (Pickups%20Location :type Vector))
  (bind _returnvalue (Transformation|GetActorTransform))
  (bind _returnvalue_2 (Math|Vector|GetForwardVector (.rotation _returnvalue)))
  (bind _returnvalue_3 (* _returnvalue_2 4e+01))
  (bind _returnvalue_4 (+ (.location _returnvalue) _returnvalue_3))
  ;[1 1 1] Spawn weapon to the hand and/or ground
  (bind _output_get (Variables|Default|SetCurrentWeaponType (.WeaponType (Utilities|GetClassDefaults WeaponToSpawn))))
  (bind (_currentweaponoftype _hasweaponoftype) (CallFunction|GetWeaponOfType _output_get))
  (if _hasweaponoftype
    (Game|SpawnActorfromClass (Variables|/Game/Props/Weapons/BP_WeaponMaster.BP_WeaponMaster_C|GetPickupClass _currentweaponoftype) (Math|Transform|MakeTransform _returnvalue_4 "0, 0, 0" "1.000000,1.000000,1.000000") "AdjustIfPossibleButAlwaysSpawn" "MultiplyWithRoot" 0 0)
    (Actor|DestroyActor _currentweaponoftype))
  (bind _returnvalue_5 (Game|SpawnActorfromClass WeaponToSpawn (Math|Transform|MakeTransform _returnvalue_4 "0, 0, 0" "1.000000,1.000000,1.000000") "AdjustIfPossibleButAlwaysSpawn" "MultiplyWithRoot" 0 0))
  (CallFunction|SetWeaponOfType (Variables|Default|GetCurrentWeaponType) _returnvalue_5)
  (Variables|Default|SetCurrentWeaponEnum (Variables|/Game/Props/Weapons/BP_WeaponMaster.BP_WeaponMaster_C|GetWeaponName _returnvalue_5))
  (Transformation|AttachComponentToComponent (Variables|/Game/Props/Weapons/BP_WeaponMaster.BP_WeaponMaster_C|GetWeaponModel _returnvalue_5) (Variables|Character|GetMesh) (Variables|/Game/Props/Weapons/BP_WeaponMaster.BP_WeaponMaster_C|GetSocket%20Name _returnvalue_5) "SnapToTarget" "SnapToTarget" "SnapToTarget" true)
  (CallFunction|SetWeaponVisibility))

(event Custom|Take%20Ammo
  (params (New%20Ammo :type Integer) (Weapon%20Type :type Enum_WeaponType%20Enum :default "NewEnumerator0"))
  ;[1 1 1] Get Ammo
  (bind _currentweaponoftype (CallFunction|GetWeaponOfType Weapon%20Type))
  (Variables|/Game/Props/Weapons/BP_WeaponMaster.BP_WeaponMaster_C|SetAmmo _currentweaponoftype (Math|Integer|Clamp(Integer) (+ New%20Ammo (Variables|/Game/Props/Weapons/BP_WeaponMaster.BP_WeaponMaster_C|GetAmmo _currentweaponoftype)) 0 (Variables|/Game/Props/Weapons/BP_WeaponMaster.BP_WeaponMaster_C|GetMaxAmmo _currentweaponoftype)))
  (Default|PlayAmmoPickupSound (Variables|Default|GetBP_Sound)))

(event Input|EnhancedActionEvents|EnhancedInputActionMy_Look
  (params (ActionValue :type Vector%202D%20Structure) (ElapsedSeconds :type Float%20%28double-precision%29) (TriggeredSeconds :type Float%20%28double-precision%29) (InputAction :type Input%20Action%20Object%20Reference :default "/Game/Player/Input/My_Look.My_Look"))
  ;[0.8717 1 0.3181] Movement
  (Pawn|Input|AddControllerYawInput (.x ActionValue))
  (Pawn|Input|AddControllerPitchInput (.y ActionValue)))

(event Input|EnhancedActionEvents|EnhancedInputActionMy_Jump
  (params (ActionValue :type Boolean) (ElapsedSeconds :type Float%20%28double-precision%29) (TriggeredSeconds :type Float%20%28double-precision%29) (InputAction :type Input%20Action%20Object%20Reference :default "/Game/Player/Input/My_Jump.My_Jump"))
  ;[0.8717 1 0.3181] Movement
  (:Started
    (Character|Jump))
  (:Completed
    (Character|StopJumping)))

(event Input|EnhancedActionEvents|EnhancedInputActionMy_SecondWeapon
  (params (ActionValue :type Boolean) (ElapsedSeconds :type Float%20%28double-precision%29) (TriggeredSeconds :type Float%20%28double-precision%29) (InputAction :type Input%20Action%20Object%20Reference :default "/Game/Player/Input/My_SecondWeapon.My_SecondWeapon"))
  ;[1 1 1] Equip weapon from inventory
  (CallFunction|EquipWeapon "NewEnumerator2"))

(event Input|EnhancedActionEvents|EnhancedInputActionMy_Reload
  (params (ActionValue :type Boolean) (ElapsedSeconds :type Float%20%28double-precision%29) (TriggeredSeconds :type Float%20%28double-precision%29) (InputAction :type Input%20Action%20Object%20Reference :default "/Game/Player/Input/My_Reload.My_Reload"))
  (bind _mesh (Variables|Character|GetMesh))
  ;[1 1 1] Reload system
  (bind _currentweapon (CallFunction|GetCurrentWeapon))
  (if (Math|Boolean|ANDBoolean (!= (Variables|/Game/Props/Weapons/BP_WeaponMaster.BP_WeaponMaster_C|GetMagasinSize _currentweapon) (Variables|/Game/Props/Weapons/BP_WeaponMaster.BP_WeaponMaster_C|GetAmmoOnMagazine _currentweapon)) (!= (Variables|/Game/Props/Weapons/BP_WeaponMaster.BP_WeaponMaster_C|GetAmmo _currentweapon) 0) (not (Variables|Default|GetIsReloading)))
    (Variables|Default|SetIsReloading true)
    (Variables|Default|SetCanFire false)
    (if (and (Variables|Default|GetIsAiming) (or (Utilities|Enum|Equal(Enum) (Variables|Default|GetCurrentWeaponType) "NewEnumerator2") (Utilities|Enum|Equal(Enum) (Variables|Default|GetCurrentWeaponType) "NewEnumerator6")))
      (Animation|Montage|PlayMontage _mesh (Variables|/Game/Props/Weapons/BP_WeaponMaster.BP_WeaponMaster_C|GetReloadAim _currentweapon) 1.4
        (:OnCompleted
          (bind _currentweapon_2 (CallFunction|GetCurrentWeapon :!label _label))
          (if (not (< (- (Variables|/Game/Props/Weapons/BP_WeaponMaster.BP_WeaponMaster_C|GetAmmo _currentweapon_2) (- (Variables|/Game/Props/Weapons/BP_WeaponMaster.BP_WeaponMaster_C|GetMagasinSize _currentweapon_2) (Variables|/Game/Props/Weapons/BP_WeaponMaster.BP_WeaponMaster_C|GetAmmoOnMagazine _currentweapon_2))) 0))
            (Variables|/Game/Props/Weapons/BP_WeaponMaster.BP_WeaponMaster_C|SetAmmo _currentweapon_2 (- (Variables|/Game/Props/Weapons/BP_WeaponMaster.BP_WeaponMaster_C|GetAmmo _currentweapon_2) (- (Variables|/Game/Props/Weapons/BP_WeaponMaster.BP_WeaponMaster_C|GetMagasinSize _currentweapon_2) (Variables|/Game/Props/Weapons/BP_WeaponMaster.BP_WeaponMaster_C|GetAmmoOnMagazine _currentweapon_2))))
            (Variables|/Game/Props/Weapons/BP_WeaponMaster.BP_WeaponMaster_C|SetAmmoOnMagazine _currentweapon_2 (Variables|/Game/Props/Weapons/BP_WeaponMaster.BP_WeaponMaster_C|GetMagasinSize _currentweapon_2))
            (else
              (Variables|/Game/Props/Weapons/BP_WeaponMaster.BP_WeaponMaster_C|SetAmmoOnMagazine _currentweapon_2 (Math|Integer|Clamp(Integer) (+ (Variables|/Game/Props/Weapons/BP_WeaponMaster.BP_WeaponMaster_C|GetAmmoOnMagazine _currentweapon_2) (Variables|/Game/Props/Weapons/BP_WeaponMaster.BP_WeaponMaster_C|GetAmmo _currentweapon_2)) 0 (Variables|/Game/Props/Weapons/BP_WeaponMaster.BP_WeaponMaster_C|GetMagasinSize _currentweapon_2)))
              (Variables|/Game/Props/Weapons/BP_WeaponMaster.BP_WeaponMaster_C|SetAmmo _currentweapon_2 0)))
          (Variables|Default|SetCanFire true)
          (Variables|Default|SetIsReloading false))
        (:OnInterrupted
          (Variables|Default|SetIsReloading false :!label _label_2)))
      (else
        (Animation|Montage|PlayMontage _mesh (Variables|/Game/Props/Weapons/BP_WeaponMaster.BP_WeaponMaster_C|GetReload _currentweapon) 1.4
          (:OnCompleted
            (goto _label))
          (:OnInterrupted
            (goto _label_2)))))))

(event Input|EnhancedActionEvents|EnhancedInputActionMy_Grapin
  (params (ActionValue :type Vector%202D%20Structure) (ElapsedSeconds :type Float%20%28double-precision%29) (TriggeredSeconds :type Float%20%28double-precision%29) (InputAction :type Input%20Action%20Object%20Reference :default "/Game/Player/Input/My_Grapin.My_Grapin"))
  (bind _returnvalue (Game|GetPlayerCameraManager 0))
  (bind _returnvalue_2 (Camera|GetCameraLocation _returnvalue))
  ;[1 0.851 0.1504] Grappin
  (:Started
    (bind (_outhit _returnvalue_3) (Collision|LineTraceForObjects _returnvalue_2 (+ _returnvalue_2 (* (Transformation|GetActorForwardVector _returnvalue) 5000)) (Utilities|Array|MakeArray "ObjectTypeQuery1") false 0 "None"))
    (if _returnvalue_3
      (Variables|Default|SetGrappinPointLocation (.ImpactPoint (Collision|BreakHitResult _outhit)))
      (Variables|Default|SetIsGrappin true)
      (Pawn|Components|CharacterMovement|SetMovementMode (Variables|Character|GetCharacterMovement) "MOVE_Flying" 0)
      (Rendering|SetVisibility (Variables|Default|GetCable) true false)))
  (:Completed
    (Variables|Default|SetIsGrappin false)
    (Pawn|Components|CharacterMovement|SetMovementMode (Variables|Character|GetCharacterMovement) "MOVE_Falling" 0)
    (Rendering|SetVisibility (Variables|Default|GetCable) false false)))

(event Input|EnhancedActionEvents|EnhancedInputActionMy_Move
  (params (ActionValue :type Vector%202D%20Structure) (ElapsedSeconds :type Float%20%28double-precision%29) (TriggeredSeconds :type Float%20%28double-precision%29) (InputAction :type Input%20Action%20Object%20Reference :default "/Game/Player/Input/My_Move.My_Move"))
  ;[0.8717 1 0.3181] Movement
  (Pawn|Input|AddMovementInput (Math|Vector|GetRightVector (Math|Rotator|MakeRotator 0.0 0.0 (.yaw (Pawn|GetControlRotation :!class /Script/Engine.Pawn)))) (.x ActionValue) false)
  (Pawn|Input|AddMovementInput (Math|Vector|GetForwardVector (Math|Rotator|MakeRotator 0.0 0.0 (.yaw (Pawn|GetControlRotation :!class /Script/Engine.Pawn)))) (.y ActionValue) false))

(event Input|EnhancedActionEvents|EnhancedInputActionMy_Aim
  (params (ActionValue :type Boolean) (ElapsedSeconds :type Float%20%28double-precision%29) (TriggeredSeconds :type Float%20%28double-precision%29) (InputAction :type Input%20Action%20Object%20Reference :default "/Game/Player/Input/My_Aim.My_Aim"))
  (bind _charactermovement (Variables|Character|GetCharacterMovement))
  (bind _charactermovement_2 (Variables|Character|GetCharacterMovement))
  ;[0.8706 1 0.3176] Aim input
  (:Started
    (Variables|Default|SetIsAiming true)
    (Variables|/Script/Engine.CharacterMovementComponent|SetbOrientRotationToMovement _charactermovement false)
    (Variables|/Script/Engine.CharacterMovementComponent|SetbUseControllerDesiredRotation _charactermovement true)
    (bind _camera_arm_lenght (Timeline|Aim Play)
      (:Update
        (Variables|/Script/Engine.SpringArmComponent|SetTargetArmLength (Variables|Default|GetSpringArm) (Math|Float|Lerp 4e+02 1.7e+02 _camera_arm_lenght)))))
  (:Completed
    (Variables|Default|SetIsAiming false)
    (Variables|/Script/Engine.CharacterMovementComponent|SetbOrientRotationToMovement _charactermovement_2 true)
    (Variables|/Script/Engine.CharacterMovementComponent|SetbUseControllerDesiredRotation _charactermovement_2 false)
    (Timeline|Aim Reverse)))

(event Input|EnhancedActionEvents|EnhancedInputActionMy_Fire
  (params (ActionValue :type Boolean) (ElapsedSeconds :type Float%20%28double-precision%29) (TriggeredSeconds :type Float%20%28double-precision%29) (InputAction :type Input%20Action%20Object%20Reference :default "/Game/Player/Input/My_Fire.My_Fire"))
  (bind _mesh (Variables|Character|GetMesh))
  (bind _currentweapontype (Variables|Default|GetCurrentWeaponType))
  (bind _camera (Variables|Default|GetCamera))
  (bind _returnvalue (Transformation|GetWorldRotation _camera))
  (bind _returnvalue_2 (Utilities|Enum|Equal(Enum) _currentweapontype "NewEnumerator6"))
  (bind _returnvalue_3 (Math|Vector|GetForwardVector _returnvalue))
  ;[1 1 1] Fire logic
  (:Triggered
    (bind _currentweapon (CallFunction|GetCurrentWeapon))
    (Utilities|IsValid _currentweapon
      (:Is%20Valid
        (if (and (Variables|Default|GetCanFire) (!= (Variables|/Game/Props/Weapons/BP_WeaponMaster.BP_WeaponMaster_C|GetAmmoOnMagazine _currentweapon) 0))
          (Utilities|FlowControl|DoOnce (!= (Variables|Default|GetCanFire) true) :!label _label
            (:Completed
              (Utilities|FlowControl|Sequence
                (:then_0
                  (Audio|PlaySound2D (Variables|/Game/Props/Weapons/BP_WeaponMaster.BP_WeaponMaster_C|GetSound _currentweapon) 1.0 1.0 0.0 0 0)
                  (if _returnvalue_2
                    (Animation|Montage|PlayMontage _mesh "/Game/Animation/AM_ShootShotgun.AM_ShootShotgun"
                      (:then
                        _))
                    (else
                      (Animation|Montage|PlayMontage _mesh "/Game/Animation/AM_Shoot.AM_Shoot"
                        (:then
                          _))))
                  (Variables|/Game/Props/Weapons/BP_WeaponMaster.BP_WeaponMaster_C|SetAmmoOnMagazine _currentweapon (- (Variables|/Game/Props/Weapons/BP_WeaponMaster.BP_WeaponMaster_C|GetAmmoOnMagazine _currentweapon) 1))
                  (Effects|SpawnEmitterAttached "/Game/InfinityBladeEffects/Effects/FX_Monsters/FX_Monster_Gruntling/Master/P_BackPack_MuzzleFlash.P_BackPack_MuzzleFlash" _mesh "Barrel" (.location (Transformation|GetSocketTransform (Variables|/Game/Props/Weapons/BP_WeaponMaster.BP_WeaponMaster_C|GetWeaponModel _currentweapon) "Barrel" "RTS_World")) _returnvalue "0.250000,0.250000,0.250000" "KeepWorldPosition" true "AutoRelease")
                  (if _returnvalue_2
                    (for _index (range 1 10)
                      (bind (_outhit _returnvalue_4) (Collision|LineTraceByChannel (+ (.location (Transformation|GetSocketTransform (Variables|/Game/Props/Weapons/BP_WeaponMaster.BP_WeaponMaster_C|GetWeaponModel _currentweapon) "Barrel" "RTS_World")) _returnvalue_3) (+ (.location (Transformation|GetSocketTransform (Variables|/Game/Props/Weapons/BP_WeaponMaster.BP_WeaponMaster_C|GetWeaponModel _currentweapon) "Barrel" "RTS_World")) (* _returnvalue_3 (Variables|/Game/Props/Weapons/BP_WeaponMaster.BP_WeaponMaster_C|GetRange _currentweapon)) (Math|Vector|MakeVector (Math|Random|RandomFloatinRange -1e+02 1e+02) (Math|Random|RandomFloatinRange -1e+02 1e+02) (Math|Random|RandomFloatinRange -1e+02 1e+02))) "TraceTypeQuery1" false 0 "ForDuration"))
                      (if _returnvalue_4
                        (Game|Damage|ApplyDamage (.HitActor (Collision|BreakHitResult _outhit)) (Variables|/Game/Props/Weapons/BP_WeaponMaster.BP_WeaponMaster_C|GetDamage _currentweapon) 0 0 "/Script/Engine.DamageType")
                        (Effects|SpawnEmitteratLocation "/Game/InfinityBladeEffects/Effects/FX_Monsters/FX_Monster_Troll/death/P_TrollDeathImpact.P_TrollDeathImpact" (.ImpactPoint (Collision|BreakHitResult _outhit)) (Math|Rotator|MakeRotfromX (.Normal (Collision|BreakHitResult _outhit))) "0.350000,0.350000,0.350000")
                        (Audio|PlaySoundatLocation "/Game/Sound/Bullet_Impact_Concrete.Bullet_Impact_Concrete" (Transformation|GetActorLocation) "0, 0, 0" 0.35 1.0 0.0 0 0 0 0)))
                    (else
                      (bind (_outhit_2 _returnvalue_5) (Collision|LineTraceByChannel (+ (.location (Transformation|GetSocketTransform (Variables|/Game/Props/Weapons/BP_WeaponMaster.BP_WeaponMaster_C|GetWeaponModel _currentweapon) "Barrel" "RTS_World")) _returnvalue_3) (+ (.location (Transformation|GetSocketTransform (Variables|/Game/Props/Weapons/BP_WeaponMaster.BP_WeaponMaster_C|GetWeaponModel _currentweapon) "Barrel" "RTS_World")) (* _returnvalue_3 (Variables|/Game/Props/Weapons/BP_WeaponMaster.BP_WeaponMaster_C|GetRange _currentweapon))) "TraceTypeQuery1" false 0 "None"))
                      (if _returnvalue_5
                        (Game|Damage|ApplyDamage (.HitActor (Collision|BreakHitResult _outhit_2)) (Variables|/Game/Props/Weapons/BP_WeaponMaster.BP_WeaponMaster_C|GetDamage _currentweapon) 0 0 "/Script/Engine.DamageType")
                        (Effects|SpawnEmitteratLocation "/Game/InfinityBladeEffects/Effects/FX_Monsters/FX_Monster_Troll/death/P_TrollDeathImpact.P_TrollDeathImpact" (.ImpactPoint (Collision|BreakHitResult _outhit_2)) (Math|Rotator|MakeRotfromX (.Normal (Collision|BreakHitResult _outhit_2))) "0.350000,0.350000,0.350000")
                        (Audio|PlaySoundatLocation "/Game/Sound/Bullet_Impact_Concrete.Bullet_Impact_Concrete" (Transformation|GetActorLocation) "0, 0, 0" 0.35 1.0 0.0 0 0 0 0)))))
                (:then_1
                  (Utilities|FlowControl|Delay (Variables|/Game/Props/Weapons/BP_WeaponMaster.BP_WeaponMaster_C|GetSpeedBullet _currentweapon))
                  (if (Utilities|Enum|NotEqual(Enum) (Variables|/Game/Props/Weapons/BP_WeaponMaster.BP_WeaponMaster_C|GetFireMode _currentweapon) "NewEnumerator0")
                    (Variables|Default|SetCanFire false)
                    (goto _label Reset)
                    (else
                      (goto _label Reset)))))))))))
  (:Started
    (CallFunction|AimForward))
  (:Completed
    (CallFunction|StopAimForward)
    (Variables|Default|SetCanFire true)))

(event Input|EnhancedActionEvents|EnhancedInputActionMy_Interact
  (params (ActionValue :type Boolean) (ElapsedSeconds :type Float%20%28double-precision%29) (TriggeredSeconds :type Float%20%28double-precision%29) (InputAction :type Input%20Action%20Object%20Reference :default "/Game/Player/Input/My_Interact.My_Interact"))
  ;[1 1 1] Get weapon from ground
  (Development|PrintText "I'm Picking up")
  (Class|WBInteract|Interact(Message) (Utilities|Array|Get(acopy) (Collision|GetOverlappingActors "/Game/Props/Pickup/BP_PickupMaster.BP_PickupMaster_C" :!class /Script/Engine.Actor)) self))

(event Input|EnhancedActionEvents|EnhancedInputActionMy_FirstWeapon
  (params (ActionValue :type Boolean) (ElapsedSeconds :type Float%20%28double-precision%29) (TriggeredSeconds :type Float%20%28double-precision%29) (InputAction :type Input%20Action%20Object%20Reference :default "/Game/Player/Input/My_FirstWeapon.My_FirstWeapon"))
  ;[1 1 1] Equip weapon from inventory
  (CallFunction|EquipWeapon "NewEnumerator1"))

(event Input|EnhancedActionEvents|EnhancedInputActionMy_ThirdWeapon
  (params (ActionValue :type Boolean) (ElapsedSeconds :type Float%20%28double-precision%29) (TriggeredSeconds :type Float%20%28double-precision%29) (InputAction :type Input%20Action%20Object%20Reference :default "/Game/Player/Input/My_ThirdWeapon.My_ThirdWeapon"))
  ;[1 1 1] Equip weapon from inventory
  (CallFunction|EquipWeapon "NewEnumerator6"))

(event Input|EnhancedActionEvents|EnhancedInputActionMy_Unarmed
  (params (ActionValue :type Boolean) (ElapsedSeconds :type Float%20%28double-precision%29) (TriggeredSeconds :type Float%20%28double-precision%29) (InputAction :type Input%20Action%20Object%20Reference :default "/Game/Player/Input/My_Unarmed.My_Unarmed"))
  ;[1 1 1] Equip weapon from inventory
  (if (Utilities|Enum|NotEqual(Enum) (Variables|Default|GetCurrentWeaponType) "NewEnumerator0")
    (Variables|Default|SetCanFire false)
    (Variables|Default|SetCurrentWeaponType "NewEnumerator0")
    (Animation|Montage|PlayMontage (Variables|Character|GetMesh) "/Game/Animation/AM_EquipRifle.AM_EquipRifle" 1.4
      (:then
        (Variables|Default|SetCurrentWeaponEnum "NewEnumerator0"))
      (:OnCompleted
        (Variables|Default|SetCanFire true))
      (:OnNotifyBegin
        (CallFunction|SetWeaponVisibility)))))

(event EventBeginPlay
  (CallFunction|SetInputMappingContext)
  (CallFunction|SetSpawnPosition)
  (Variables|Default|SetLife (Variables|Default|GetMaxLife)))

(event EventTick
  (params (DeltaSeconds :type Float%20%28single-precision%29))
  ;[1 0.851 0.1504] Grappin
  (if (Variables|Default|GetIsGrappin)
    (Physics|AddForce (Variables|Character|GetCharacterMovement) (* (Math|Vector|GetUnitDirection(Vector) (Transformation|GetActorLocation) (Variables|Default|GetGrappinPointLocation)) 300000))
    (Variables|/Script/CableComponent.CableComponent|SetEndLocation (Variables|Default|GetCable) (Math|Transform|InverseTransformLocation (Transformation|GetActorTransform) (Variables|Default|GetGrappinPointLocation)))
    (if (<= (Math|Vector|Distance(Vector) (Variables|Default|GetGrappinPointLocation) (Transformation|GetActorLocation)) 1e+02)
      (Variables|Default|SetIsGrappin false)
      (Pawn|Components|CharacterMovement|SetMovementMode (Variables|Character|GetCharacterMovement) "MOVE_Falling" 0)
      (Rendering|SetVisibility (Variables|Default|GetCable) false false))))

(fn ConstructionScript)

(fn GetCurrentWeapon
  (bind _currentweaponoftype (CallFunction|GetWeaponOfType (Variables|Default|GetCurrentWeaponType)))
  (return _currentweaponoftype))

(fn GetWeaponOfType
  (params (WeaponType :type Enum_WeaponType%20Enum :default "NewEnumerator0"))
  (bind _weapons (Variables|Default|GetWeapons))
  (bind (_value _returnvalue) (Utilities|Map|Find _weapons WeaponType))
  (return _value _returnvalue))

(fn SetWeaponOfType
  (params (WeaponType :type Enum_WeaponType%20Enum :default "NewEnumerator0") (WeaponToSet :type BP%20Weapon%20Master%20Object%20Reference))
  (Utilities|Map|Add (Variables|Default|GetWeapons) WeaponType WeaponToSet))

(fn SetWeaponVisibility
  (bind _weapons (Variables|Default|GetWeapons))
  (bind _keys (Utilities|Map|Keys _weapons))
  (for _array_element _keys
    (if (Utilities|Enum|NotEqual(Enum) _array_element (Variables|Default|GetCurrentWeaponType))
      (Utilities|IsValid (.Value (Utilities|Map|Find _weapons _array_element))
        (:Is%20Valid
          (Rendering|SetVisibility (Variables|/Game/Props/Weapons/BP_WeaponMaster.BP_WeaponMaster_C|GetWeaponModel (.Value (Utilities|Map|Find _weapons _array_element))) false false)))
      (else
        (Utilities|IsValid (.Value (Utilities|Map|Find _weapons _array_element))
          (:Is%20Valid
            (Rendering|SetVisibility (Variables|/Game/Props/Weapons/BP_WeaponMaster.BP_WeaponMaster_C|GetWeaponModel (.Value (Utilities|Map|Find _weapons _array_element))) true false)))))))

(fn TakeWeapon
  (params (NewWeapon :type Enum_WeaponType%20Enum :default "NewEnumerator0"))
  (bind _hasweaponoftype (CallFunction|GetWeaponOfType NewWeapon))
  (if (and _hasweaponoftype (Utilities|Enum|NotEqual(Enum) (Variables|Default|GetCurrentWeaponType) NewWeapon))
    (Variables|Default|SetCanFire false)
    (Variables|Default|SetCurrentWeaponType NewWeapon)
    (return true)
    (else
      (return false))))

(fn RandomValue
  (params (Socket :type Vector) (Camera :type Vector))
  (return "0, 0, 0"))