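; Wave manager for the zombie mode on the snowy village level, running timed rounds from an intro cinematic through to victory.
; Each round sets a zombie quota that scales with round number, then a looping timer triggers every BP_EnemySpawner while under the alive cap.
; CheckRoundEnd, not called within this Blueprint, advances once all zombies are dead.
; After round five it plays the win cinematic, pauses and shows WB_Win.
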(event Custom|Increase%20Round
  ;[1 0.4352 0] Increase round
  (Math|Integer|IncrementInt (Variables|Default|GetRound_NB)
    (:%20%20
      (Utilities|FlowControl|Delay (Variables|Default|GetTime_Between_Round))
      (CallFunction|StartRound))))

(event Custom|Start%20Round
  (bind _round_nb (Variables|Default|GetRound_NB))
  ;[1 0.4674 0] Spawn
  (Variables|Default|SetTotal_Zombies_In_Round (Math|Integer|SelectInt (Math|Float|Round (* (* (Variables|Default|GetRound_NB) 0.15) (Variables|Default|GetMax_Zombies_In_Level))) (Math|Integer|SelectInt 6 9 (== _round_nb 1)) (> _round_nb 2)))
  (Utilities|FlowControl|Delay 0.5)
  (bind _returnvalue (Utilities|Time|SetTimerbyEvent (delegate Custom|Spawn%20Zombie) (Variables|Default|GetTime_Between_Spawn) true)))

(event Custom|Level%20sequence
  (params (LevelS :type Level%20Sequence%20Object%20Reference))
  (bind _returnvalue (Sequencer|Player|CreateLevelSequencePlayer LevelS))
  (Sequencer|Player|Play _returnvalue :!class /Script/MovieScene.MovieSceneSequencePlayer)
  (CallFunction|DisableControl))

(event Custom|Spawn%20Zombie
  ;[1 0.4674 0] Spawn
  (if (< (Variables|Default|GetZombies_Spawned) (Variables|Default|GetTotal_Zombies_In_Round))
    (if (<= (Variables|Default|GetZombies_Alive) (Variables|Default|GetMax_Zombies_In_Level))
      (CallFunction|Spawn))
    (else
      ;;[1 1 1] Check round end
      (Utilities|Time|ClearandInvalidateTimerbyHandle (stale Custom|Start%20Round _returnvalue)))))

(event Custom|Check%20round%20end
  ;[1 1 1] Check round end
  (Utilities|FlowControl|Delay 0.1)
  (if (and (>= (Variables|Default|GetZombies_Spawned) (Variables|Default|GetTotal_Zombies_In_Round)) (== (Variables|Default|GetZombies_Alive) 0))
    (Variables|Default|SetZombies_Spawned 0)
    (if (> (+ (Variables|Default|GetRound_NB) 1) 5)
      (Audio|PlaySound2D "/Game/Music/victory-epic-music-155790.victory-epic-music-155790" 1.0 1.0 0.0 0 0)
      (CallFunction|LevelSequence "/Game/Sequence/LSP_WinVillageSnow.LSP_WinVillageSnow")
      (CallFunction|DisableControl)
      (Utilities|FlowControl|Delay 1e+01)
      (Game|SetGamePaused true)
      (bind _returnvalue (UserInterface|CreateWidget "/Game/Player/UserInterface/WB_Win.WB_Win_C" (Game|GetPlayerController 0)))
      (UserInterface|Viewport|AddtoViewport _returnvalue 0)
      (else
        (CallFunction|IncreaseRound)
        ;[1 0.4674 0] Spawn
        (Utilities|Time|ClearandInvalidateTimerbyHandle (stale Custom|Start%20Round _returnvalue))))))

(event Custom|Disable%20Control
  (bind _returnvalue (Game|GetPlayerController 0))
  (Input|SetIgnoreMoveInput _returnvalue true)
  (Input|SetIgnoreLookInput _returnvalue true)
  (Input|DisableInput _returnvalue _returnvalue))

(event Custom|Enable%20control
  (bind _returnvalue (Game|GetPlayerController 0))
  (Input|SetIgnoreMoveInput _returnvalue false)
  (Input|SetIgnoreLookInput _returnvalue false)
  (Input|EnableInput (Game|GetPlayerCharacter 0) _returnvalue))

(event EventBeginPlay
  (CallFunction|LevelSequence "/Game/Sequence/LSP_VillageSnow.LSP_VillageSnow")
  (Utilities|FlowControl|Delay 1e+01)
  (CallFunction|EnableControl)
  (CallFunction|CheckNumberOfSpawner)
  (CallFunction|IncreaseRound))

(fn ConstructionScript)

(fn Spawn
  (bind _outactors (Actor|GetAllActorsOfClass "/Game/Enemy/BP_EnemySpawner.BP_EnemySpawner_C"))
  (for _array_element _outactors
    (Default|Spawn _array_element)
    (Math|Integer|IncrementInt (Variables|Default|GetZombies_Spawned)
      (:%20%20
        (Math|Integer|IncrementInt (Variables|Default|GetZombies_Alive))))))

(fn CheckNumberOfSpawner
  (bind _outactors (Actor|GetAllActorsOfClass "/Game/Enemy/BP_EnemySpawner.BP_EnemySpawner_C"))
  (Variables|Default|SetMulitplier (Utilities|Array|Length _outactors)))